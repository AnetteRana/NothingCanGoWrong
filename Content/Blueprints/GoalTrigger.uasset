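; Goal actor for a golf game that ends the game when the ball overlaps it.
; Two seconds after BeginPlay it caches the GolfGameMode and its ball reference, then calls WhenGameOver on that game mode when the ball enters.
; Tick spins the cube in yaw and bobs it by adding a sine offset to its Z each frame, so the bob is frame-rate dependent.
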(event `self.ReceiveBeginPlay`
  (`KismetSystemLibrary.Delay` 2.0)
  (bind _asgolf_game_mode (cast `/Game/Core/GolfGameMode` (`GameplayStatics.GetGameMode`)))
  (`/Engine/EditorBlueprintResources/StandardMacros.IsValid` _asgolf_game_mode
    (:`Is Valid`
      (bind _output_get (set `self.As Golf Game Mode` _asgolf_game_mode))
      (set `self.Ball Ref` (`/Game/Core/GolfGameMode.ballRef` _output_get)))))

(event `self.ReceiveTick`
  (params (DeltaSeconds :type "Float (single-precision)"))
  (bind _cube (`self.Cube`))
  (bind _output_get (set `self.Time` (+ (stale _output_get) DeltaSeconds)))
  (`SceneComponent.K2_AddRelativeRotation` _cube (`KismetMathLibrary.MakeRotator` 0.0 0.0 (* DeltaSeconds (`self.RotatePerSecond`))) false false)
  (`SceneComponent.K2_SetRelativeLocation` _cube (`KismetMathLibrary.MakeVector` (.x (`SceneComponent.RelativeLocation` _cube)) (.y (`SceneComponent.RelativeLocation` _cube)) (+ (.z (`SceneComponent.RelativeLocation` _cube)) (/ (`KismetMathLibrary.Sin` (* (`self.Time`) 1.0)) 2.0))) false false))

(event `self.ReceiveActorBeginOverlap`
  (params (OtherActor :type "Actor Object Reference"))
  (if (== OtherActor (`self.Ball Ref`))
    (`/Game/Core/GolfGameMode.WhenGameOver` (`self.As Golf Game Mode`))))

(fn `UserConstructionScript`)