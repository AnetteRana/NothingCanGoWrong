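; Player camera pawn for a golf game that handles aiming and hitting the ball, and creates the HUD and pause menu.
; It registers with GolfGameMode, follows the ball while attached, and rotates its spring arm and moves the golfer on input.
; Holding the hit input ping-pongs power between limits on Tick.
; Release applies a lofted impulse along camera forward, then locks hitting until WhenReadyToHitBall re-enables it.
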(event `WhenReadyToHitBall`
  ; rotate around enabled until click
  (set `self.isMyHittingEnabled` true))

(event `ballReceiveHit`
  (bind _currenthitstrength (`self.currentHitStrength`))
  ; rotate around enabled until click
  (`PrimitiveComponent.AddImpulse` (`/Game/Blueprints/TheBall.BallMesh` (`self.ballRef`)) (`KismetMathLibrary.MakeVector` (.x (* (`KismetMathLibrary.Normal` (`SceneComponent.GetForwardVector` (`self.TheCamera`))) (* _currenthitstrength 0.5))) (.y (* (`KismetMathLibrary.Normal` (`SceneComponent.GetForwardVector` (`self.TheCamera`))) (* _currenthitstrength 0.5))) (* _currenthitstrength 0.5)) "None" false))

(event `self.ReceiveBeginPlay`
  ;[1 0.9425 0 0.5] BeginPlay
  (`|ExecutionSequence`
    (:`then_0`
      (bind _asgolf_game_mode (cast `/Game/Core/GolfGameMode` (`GameplayStatics.GetGameMode`)))
      (`/Engine/EditorBlueprintResources/StandardMacros.IsValid` _asgolf_game_mode
        (:`Is Valid`
          (set `/Game/Core/GolfGameMode.playerCameraRef` self _asgolf_game_mode)
          (set `self.GM_ref` _asgolf_game_mode)
          (`KismetSystemLibrary.Delay` 0.2)
          (set `self.ballRef` (`/Game/Core/GolfGameMode.ballRef` (`self.GM_ref`))))))
    (:`then_1`
      (bind _returnvalue (`|CreateWidget` "/Game/UI/W_HUD.W_HUD_C" (`GameplayStatics.GetPlayerController` 0)))
      (set `/Game/Core/GolfGameMode.playerUI` _returnvalue (`self.GM_ref`))
      (`UserWidget.AddToViewport` _returnvalue 0))
    (:`then_2`
      (`EnhancedInputSubsystemInterface.AddMappingContext` (pcsubsystem `EnhancedInputLocalPlayerSubsystem` (`GameplayStatics.GetPlayerController` 0)) "/Game/Input/IMC_PlayerControls.IMC_PlayerControls" 0 (struct)))))

(event `Key|One`
  (params (Key :type "Key Structure"))
  (bind _returnvalue (`GameplayStatics.GetPlayerController` 0))
  ; pause menu
  (:`Pressed`
    (bind _returnvalue_2 (`|CreateWidget` "/Game/UI/W_pauseScreen.W_pauseScreen_C" _returnvalue :!label _label))
    (`WidgetBlueprintLibrary.SetInputMode_UIOnlyEx` _returnvalue _returnvalue_2)
    (`GameplayStatics.SetGamePaused` true)
    (`UserWidget.AddToViewport` _returnvalue_2 0)))

(event `Key|Escape`
  (params (Key :type "Key Structure"))
  ; pause menu
  (:`Pressed`
    (goto _label)))

(event `self.ReceiveTick`
  (params (DeltaSeconds :type "Float (single-precision)"))
  (bind _ballref (`self.ballRef`))
  ;[0 0.7372 1 0.5] Tick
  (`|ExecutionSequence`
    (:`then_0`
      (set `self.Delta Seconds` DeltaSeconds)
      (if (`/Game/Core/GolfGameMode.isCameraAttachedToBall` (`self.GM_ref`))
        (`/Engine/EditorBlueprintResources/StandardMacros.IsValid` _ballref
          (:`Is Valid`
            (`self.K2_SetActorLocation` (`SceneComponent.K2_GetComponentLocation` (`Actor.RootComponent` _ballref))))))
      (if (`self.isCharging`)
        (`self.OscillatePower`)))))

(event `EnhancedInput|/Game/Input/IA_RotateCamera`
  (params (ActionValue :type "Float (double-precision)") (ElapsedSeconds :type "Float (double-precision)") (TriggeredSeconds :type "Float (double-precision)") (InputAction :type "InputAction Object Reference" :default "/Game/Input/IA_RotateCamera.IA_RotateCamera"))
  ; A and D = rotate
  (:`Triggered`
    (set `/Game/Blueprints/TheGolfer.strafingDirection` ActionValue (`/Game/Core/GolfGameMode.golferCharRef` (`self.GM_ref`)))
    (if (`self.isMyHittingEnabled`)
      (`SceneComponent.K2_SetWorldRotation` (`self.SpringArm`) (`KismetMathLibrary.MakeRotator` (.roll (`SceneComponent.K2_GetComponentRotation` (`self.SpringArm`))) (.pitch (`SceneComponent.K2_GetComponentRotation` (`self.SpringArm`))) (+ (.yaw (`SceneComponent.K2_GetComponentRotation` (`self.SpringArm`))) (* (`self.rotationStrength`) ActionValue))) false false)
      (`/Game/Blueprints/TheGolfer.moveGolfer` (`/Game/Core/GolfGameMode.golferCharRef` (`self.GM_ref`)) ActionValue))))

(event `EnhancedInput|/Game/Input/IA_ChargeHit`
  (params (ActionValue :type Boolean) (ElapsedSeconds :type "Float (double-precision)") (TriggeredSeconds :type "Float (double-precision)") (InputAction :type "InputAction Object Reference" :default "/Game/Input/IA_ChargeHit.IA_ChargeHit"))
  ; spacebar = hit
  (:`Started`
    (if (`self.isMyHittingEnabled`)
      (set `self.isCharging` true)
      (set `self.currentHitStrength` (`self.minHitStrength`))
      (set `self.chargeGrowthDirection` 1.0)))
  (:`Completed`
    (if (`self.isMyHittingEnabled`)
      (set `self.isCharging` false)
      (`self.ballReceiveHit`)
      (set `self.isMyHittingEnabled` false)
      (`/Game/Core/GolfGameMode.BallHasBeenHit` (`self.GM_ref`))
      (`GameplayStatics.PlaySoundAtLocation` "/Game/Audio/BallHit_Cue.BallHit_Cue" (`self.K2_GetActorLocation`) (struct) 1.0 1.0 0.0 null null null null))))

(event `OscillatePower`
  ; charge power up/down
  (bind _output_get (set `self.currentHitStrength` (+ (stale _output_get) (* (`self.chargingSpeed`) (`self.Delta Seconds`) (`self.chargeGrowthDirection`)))))
  (if (== (`self.chargeGrowthDirection`) 1.0)
    (if (>= (`self.currentHitStrength`) (`self.maxHitStrength`))
      (set `self.chargeGrowthDirection` -1.0))
    (elif (<= (`self.currentHitStrength`) (`self.minHitStrength`))
      (set `self.chargeGrowthDirection` 1.0))))

(fn `UserConstructionScript`)