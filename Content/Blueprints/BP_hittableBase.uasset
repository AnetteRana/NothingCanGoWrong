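; BP_hittableBase is a base Blueprint for objects that the ball can hit.
; A static mesh hit stores the other actor's velocity as the ball speed and plays the object's sound if valid, without checking the actor's type.
; Reusable objects respond to every hit, while others respond only to the first.
; WhenHitByBall separately fires the empty OnHitByBall event, and the hit handler calls neither.
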(event `self.StaticMesh.OnComponentHit`
  (params (HitComponent :type "PrimitiveComponent Object Reference") (OtherActor :type "Actor Object Reference") (OtherComp :type "PrimitiveComponent Object Reference") (NormalImpulse :type "Vector Structure") (Hit :type "HitResult Structure (by ref)"))
  (bind _mysound (`self.mySound`))
  (if (`self.isReusable`)
    (set `self.BallSpeedOnHit` (`self.GetVelocity` OtherActor) :!label _label)
    (`/Engine/EditorBlueprintResources/StandardMacros.IsValid` _mysound
      (:`Is Valid`
        (`AudioComponent.Play` _mysound 0.0)
        (`self.onHitByBall`)))
    (elif (not (`self.isUsedBefore`))
      (set `self.isUsedBefore` true)
      (goto _label))))

(event `onHitByBall`)

(fn `UserConstructionScript`)