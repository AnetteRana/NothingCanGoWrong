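; Hittable crow actor that flies away when struck by a ball.
; OnHitbyBall switches the skeletal mesh to the crow fly animation and plays a timeline that raises it.
; Each update lerps from the mesh's current location toward 200 units above it, so the climb accumulates rather than ending at a fixed height.
; When the timeline finishes, only the mesh component is destroyed, not the actor.
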(event `self.onHitByBall`
  (bind _skeletalmesh (`self.SkeletalMesh`))
  (bind _returnvalue (`SceneComponent.K2_GetComponentLocation` (`self.SkeletalMesh`)))
  (`SkeletalMeshComponent.SetAnimation` (`self.SkeletalMesh`) "/Game/Assets/Crow/Animations/ANIM_Crow_Fly.ANIM_Crow_Fly")
  (bind (_direction _mylerptimeline) (`Timeline|Timeline` :!via `PlayFromStart`)
    (:`Update`
      (`SceneComponent.K2_SetWorldLocation` _skeletalmesh (`KismetMathLibrary.VLerp` _returnvalue (+ _returnvalue (0.0 0.0 200.0)) _mylerptimeline) false false))
    (:`Finished`
      (`ActorComponent.K2_DestroyComponent` _skeletalmesh))))

(fn `UserConstructionScript`
  (`parent.UserConstructionScript`))