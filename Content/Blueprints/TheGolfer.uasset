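; Golfer pawn that walks to the golf ball and repositions around it relative to the player camera, using AI MoveTo.
; On BeginPlay it registers itself with GolfGameMode and keeps that reference.
; GoToBall is gated by a DoOnce, which resets after notifying the game mode on arrival.
; Strafe targets a point at the current ball distance along the camera spring arm's right vector, briefly setting StrafingDirection.
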(event `self.ReceiveBeginPlay`
  (bind _asgolf_game_mode (cast `/Game/Core/GolfGameMode` (`GameplayStatics.GetGameMode`)))
  (`/Engine/EditorBlueprintResources/StandardMacros.IsValid` _asgolf_game_mode
    (:`Is Valid`
      (set `/Game/Core/GolfGameMode.golferCharRef` self _asgolf_game_mode)
      (set `self.GM_ref` _asgolf_game_mode))))

(event `GoToBall`
  (bind _ballref (`self.BallRef`))
  (`/Engine/EditorBlueprintResources/StandardMacros.DoOnce` false :!label _label
    (:`Completed`
      (`/Engine/EditorBlueprintResources/StandardMacros.IsValid` _ballref
        (:`Is Valid`
          (`|AIMoveTo` self (0.0 0.0 0.0) _ballref 20.0 true
            (:`OnSuccess`
              (`/Game/Core/GolfGameMode.GolferFoundBall` (`self.GM_ref`))
              (goto _label :!via `Reset`))
            (:`OnFail`
              (`KismetSystemLibrary.PrintString` "ball is where???"))))))))

(event `self.ReceiveTick`
  (params (DeltaSeconds :type "Float (single-precision)")))

(event `strafe`
  (params (sideValue :type "Float (double-precision)"))
  (set `self.DistanceToBall` (`KismetMathLibrary.Vector_Distance` (`SceneComponent.K2_GetComponentLocation` (`Actor.RootComponent` (`self.BallRef`))) (`SceneComponent.K2_GetComponentLocation` (`self.CapsuleComponent`))))
  (set `self.strafingDirection` sideValue)
  (`|AIMoveTo` self (- (`SceneComponent.K2_GetComponentLocation` (`Actor.RootComponent` (`self.BallRef`))) (* (`self.DistanceToBall`) (`SceneComponent.GetRightVector` (`/Game/Blueprints/ThePlayerCamera.SpringArm` (`/Game/Core/GolfGameMode.playerCameraRef` (`self.GM_ref`)))))) null 0.1
    (:`then`
      (`KismetSystemLibrary.Delay` 0.2)
      (set `self.strafingDirection` 0.0))
    (:`OnSuccess`)
    (:`OnFail`)))

(fn `UserConstructionScript`)